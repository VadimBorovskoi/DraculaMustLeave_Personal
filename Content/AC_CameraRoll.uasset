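; Actor component that rolls the player's first-person camera according to sideways movement.
; On BeginPlay it finds player 0's camera tagged "FPSCam", caches max movement speed and turns off the camera's pawn control rotation.
; Each tick, lateral velocity as a fraction of max speed sets a clamped target roll, which FInterpTo eases toward.
; It copies pitch from the controller's control rotation and keeps the camera's relative yaw.
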(event `self.ReceiveBeginPlay`
  (`|ExecutionSequence`
    (:`then_0`
      (bind _output_get (set `self.Player` (`GameplayStatics.GetPlayerPawn` 0)))
      (set `self.MovementComponent` (`Pawn.GetMovementComponent` _output_get))
      (set `self.Camera` (`|GetArrayItem` (`Actor.GetComponentsByTag` (`self.Player`) "/Script/Engine.CameraComponent" "FPSCam")))
      (set `self.MaxSpeed` (`MovementComponent.GetMaxSpeed` (`self.MovementComponent`))))
    (:`then_1`
      (set `CameraComponent.bUsePawnControlRotation` false (`self.Camera`)))))

(event `self.ReceiveTick`
  (params (DeltaSeconds :type "Float (single-precision)"))
  (set `self.Delta Seconds` DeltaSeconds)
  (`|ExecutionSequence`
    (:`then_0`
      (set `self.LateralVelocity` (`self.PercentileVelocity`))
      ;[0.006607 0.00411 0.08333] Update Current rotation Var
      (set `self.CurrentRotation` (`SceneComponent.RelativeRotation` (`self.Camera`))))
    (:`then_1`
      (bind (_returnvalue _outputpin _outputpin2) (`self.CalculateNewRotation`))
      (`SceneComponent.K2_SetRelativeRotation` (`self.Camera`) (`KismetMathLibrary.MakeRotator` _returnvalue _outputpin _outputpin2) false false))))

(fn `CalculateNewRotation`
  (returns (ReturnValue :type "Float (double-precision)") (OutputPin :type "Float (double-precision)") (OutputPin2 :type "Float (double-precision)"))
  (bind (_returnvalue_roll _returnvalue_pitch) (`KismetMathLibrary.BreakRotator` (`Controller.GetControlRotation` (`Pawn.GetController` (`self.Player`)))))
  (bind (_returnvalue_roll_2 _returnvalue_pitch_2 _returnvalue_yaw) (`KismetMathLibrary.BreakRotator` (`KismetMathLibrary.MakeRotator` (.roll (`self.CurrentRotation`)) _returnvalue_pitch (.yaw (`self.CurrentRotation`)))))
  (return (`KismetMathLibrary.FInterpTo` _returnvalue_roll_2 (`self.CalculateAngle` (`self.PercentileVelocity`)) (`self.Delta Seconds`) (`self.InterpSpeed`)) _returnvalue_pitch_2 _returnvalue_yaw))