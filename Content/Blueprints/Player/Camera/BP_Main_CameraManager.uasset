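; Player camera manager that turns look input into yaw and pitch on the controlled pawn, switching between free and lock-on aim.
; ProcessInput selects CBPLockAim when given a valid target, otherwise CBPFreeAim, then feeds the active aim's HandleAim results to the pawn.
; A game-state reset event restores free aim.
; GetCameraManager returns itself; the other getters are empty, and the debug widget creation is disconnected.
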(event `self.ReceiveBeginPlay`
  (add `/Game/Blueprints/_Core/BP_GameState_Main.OnGameReset` (`/Game/Blueprints/_Core/References/BPFL_References.GetMainGameState`) (delegate `/Game/TestingContent/BPI_Resettable.Reset`))
  (if (`self.ShouldDebug`)
    _))

(event `/Game/TestingContent/BPI_Resettable.Reset`
  (set `self.ActiveAim` (`self.CBP_FreeAim`)))

(event `ProcessInput`
  (params (InputX :type "Float (double-precision)") (InputY :type "Float (double-precision)") (PossibleTarget :type "Actor Object Reference"))
  (bind _returnvalue (`Controller.K2_GetPawn` (`/Game/Blueprints/_Core/References/BPFL_References.GetMainPlayerController`)))
  (bind (_yawinput _pitchinput) (`/Game/Blueprints/Player/Camera/CBP_AbsAim.HandleAim` (`self.ActiveAim`) InputX InputY PossibleTarget))
  ; Switch Camera Modes
  (if (not (`KismetSystemLibrary.IsValid` PossibleTarget))
    (set `self.ActiveAim` (`self.CBP_FreeAim`))
    (else
      (set `self.ActiveAim` (`self.CBP_LockAim`))))
  (`Pawn.AddControllerYawInput` _returnvalue _yawinput)
  (`Pawn.AddControllerPitchInput` _returnvalue _pitchinput))

(fn `GetCameraManager`
  (returns (CameraManager :type "/Game/Blueprints/Player/Camera/BP_Main_CameraManager Object Reference"))
  (return self))

(fn `GetGameState`
  (returns (GameState :type "/Game/Blueprints/_Core/BP_GameState_Main Object Reference"))
  (return null))

(fn `GetPlayerCharacter`
  (params (PlayerController :type "PlayerController Object Reference"))
  (returns (Character :type "/Game/Blueprints/Player/Pawn/BP_Main_Character Object Reference"))
  (return null))

(fn `GetPlayerController`
  (returns (PlayerController :type "/Game/Blueprints/Player/BP_PlayerController_Main Object Reference"))
  (return null))

(fn `UserConstructionScript`)