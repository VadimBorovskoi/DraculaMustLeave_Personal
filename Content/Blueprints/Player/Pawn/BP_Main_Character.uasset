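; Main player character that turns input into movement and switches between basic and strafe movement based on target availability.
; Each input update selects a movement component by target validity, then feeds its returned directions and scales into AddMovementInput.
; It binds to the main game state's reset event, with a Reset handler that restores basic movement.
; GetPlayerCharacter returns itself for its own controller, while the other getters are empty stubs.
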(event `self.ReceiveBeginPlay`
  (add `/Game/Blueprints/_Core/BP_GameState_Main.OnGameReset` (`/Game/Blueprints/_Core/References/BPFL_References.GetMainGameState`) (delegate `/Game/TestingContent/BPI_Resettable.Reset`)))

(event `/Game/TestingContent/BPI_Resettable.Reset`
  (set `self.ActiveMovement` (`self.CBP_BasicMovement`)))

(event `ProcessInput`
  (params (InputX :type "Float (double-precision)") (InputY :type "Float (double-precision)") (PossibleTarget :type "Actor Object Reference"))
  (bind (_xscale _yscale _xdirection _ydirection) (`/Game/Blueprints/Player/Pawn/CBP_AbsMovement.HandleMovement` (`self.ActiveMovement`) InputX InputY PossibleTarget))
  ; Switch Movement Modes Depending on the Target Availability
  (if (not (`KismetSystemLibrary.IsValid` PossibleTarget))
    (set `self.ActiveMovement` (`self.CBP_BasicMovement`))
    (else
      (set `self.ActiveMovement` (`self.CBP_StrafeMovement`))))
  (`self.AddMovementInput` _xdirection _xscale)
  (`self.AddMovementInput` _ydirection _yscale))

(fn `GetCameraManager`
  (returns (CameraManager :type "/Game/Blueprints/Player/Camera/BP_Main_CameraManager Object Reference"))
  (return null))

(fn `GetCoreCameraManager`
  (returns (CameraManager :type "CoreCameraManager Object Reference"))
  (return null))

(fn `GetGameState`
  (returns (GameState :type "/Game/Blueprints/_Core/BP_GameState_Main Object Reference"))
  (return null))

(fn `GetPlayerCharacter`
  (params (PlayerController :type "PlayerController Object Reference"))
  (returns (Character :type "/Game/Blueprints/Player/Pawn/BP_Main_Character Object Reference"))
  (if (== PlayerController (`self.GetController`))
    (return self)))

(fn `GetPlayerController`
  (returns (PlayerController :type "/Game/Blueprints/Player/BP_PlayerController_Main Object Reference"))
  (return null))

(fn `UserConstructionScript`)