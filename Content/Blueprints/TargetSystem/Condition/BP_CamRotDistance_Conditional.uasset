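; Target system condition that scores a potential target by how closely it lines up with the sender's facing direction.
; IsFulfilled takes the angle between the sender actor's forward vector and the direction to the target component's owner.
; It normalizes that angle over 180 degrees and inverts it, so 1 is dead ahead and 0 is directly behind.
; Despite the CamRot name, it reads no camera rotation.
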(fn `IsFulfilled`
  (params (PotentialTarget :type "/Game/Blueprints/TargetSystem/Target/CBP_Target_Combat Object Reference") (Sender :type "Actor Object Reference"))
  (returns (`From 0 To 1` :type "Float (double-precision)"))
  (locals (Direction :type "Vector Structure"))
  (return (- 1.0 (/ (`KismetMathLibrary.DegAcos` (`KismetMathLibrary.Dot_VectorVector` (`Actor.GetActorForwardVector` (`local.Sender`)) (`KismetMathLibrary.Normal` (- (`Actor.K2_GetActorLocation` (`ActorComponent.GetOwner` PotentialTarget)) (`Actor.K2_GetActorLocation` Sender))))) 180.0))))