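; BP_ConditionDA is a condition asset in the target system, pairing condition data entries with instantiated condition objects.
; Initialize clears the object list and constructs one object from the Condition class in each data entry.
; GetConditions returns both arrays, first rebuilding the objects if the cache is empty or its length differs from the data's.
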(event `Initialize`
  (`KismetArrayLibrary.Array_Clear` (`self.ConditionObjects`))
  (for _array_element (`self.ConditionData`)
    (bind _returnvalue (`|GenericCreateObject` (`.Condition_17_53AF667844C006F2B452BE9A56649FDA` (break `/Game/Blueprints/TargetSystem/Condition/Str_Target_Condition` _array_element))))
    (`KismetArrayLibrary.Array_Add` (`self.ConditionObjects`) _returnvalue)))

(fn `GetConditions`
  (returns (ConditionData :type "Array of /Game/Blueprints/TargetSystem/Condition/Str_Target_Condition Structure") (ConditionActions :type "Array of /Game/Blueprints/TargetSystem/Condition/ABP_AbsTarget_Conditional Object Reference"))
  (if (or (`KismetArrayLibrary.Array_IsEmpty` (`self.ConditionObjects`)) (!= (`KismetArrayLibrary.Array_Length` (`self.ConditionObjects`)) (`KismetArrayLibrary.Array_Length` (`self.ConditionData`))))
    (`self.Initialize`))
  (return (`self.ConditionData`) (`self.ConditionObjects`)))