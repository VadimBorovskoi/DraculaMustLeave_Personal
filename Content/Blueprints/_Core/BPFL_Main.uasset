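; BPFL_Main is a core Blueprint function library of small transform and angle helpers.
; IsDefaultTransform checks a transform for zero location, zero rotation and unit scale with zero tolerance.
; GetDefaultTransform builds a transform from Pos, Rot and Scale values.
; GetNormalizedAngle is a stub that ignores its input and always returns zero.
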(fn `GetDefaultTransform`
  (returns (EmptyTransform :type "Transform Structure"))
  (locals (Pos :type "Vector Structure") (Rot :type "Rotator Structure") (Scale :type "Vector Structure" :default (1.0 1.0 1.0)))
  (return (`KismetMathLibrary.MakeTransform` (`local.Pos`) (`local.Rot`) (`local.Scale`))))

(fn `GetNormalizedAngle`
  (params (Angle :type "Float (double-precision)"))
  (returns (Normalized :type "Float (double-precision)"))
  (return 0.0))

(fn `IsDefaultTransform`
  (params (ToCheck :type "Transform Structure"))
  (returns (IsDefault :type Boolean))
  (return (and (== (.location ToCheck) (0.0 0.0 0.0)) (== (.rotation ToCheck) (struct)) (== (.scale ToCheck) (1.0 1.0 1.0)))))