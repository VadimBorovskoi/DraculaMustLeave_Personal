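; BP_PlayerHUD manages the player's main screens: the Reaper HUD, the pause screen and the game over screen.
; On BeginPlay it creates all three widgets once for the main player controller and stores them.
; Each display event clears all widgets, then adds its stored widget to the viewport, so screens replace one another.
; The game over event also initializes its widget with the player's score.
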(event `self.ReceiveBeginPlay`
  (bind _playercontroller (`/Game/Blueprints/_Core/References/BPFL_References.GetMainPlayerController`))
  (`parent.ReceiveBeginPlay`)
  (bind _returnvalue (`|CreateWidget` "/Game/UI/WBP_ReaperHUD.WBP_ReaperHUD_C" _playercontroller))
  (set `self.WidgetHUD` _returnvalue)
  (bind _returnvalue_2 (`|CreateWidget` "/Game/TestingContent/WBP_Pause.WBP_Pause_C" _playercontroller))
  (set `self.WidgetPause` _returnvalue_2)
  (bind _returnvalue_3 (`|CreateWidget` "/Game/TestingContent/WBP_GameOver.WBP_GameOver_C" _playercontroller))
  (set `self.WidgetGameOver` _returnvalue_3))

(event `self.DisplayGameOver`
  (params (FinalScore :type Integer))
  (bind _widgetgameover (`self.WidgetGameOver`))
  (`WidgetLayoutLibrary.RemoveAllWidgets`)
  (`UserWidget.AddToViewport` _widgetgameover 0)
  (`/Game/TestingContent/WBP_GameOver.Initialize` _widgetgameover (`/Game/Blueprints/_Core/References/BPFL_References.GetPlayerScore`)))

(event `self.DisplayPauseScreen`
  (params (CurrentScore :type Integer))
  (`WidgetLayoutLibrary.RemoveAllWidgets`)
  (`UserWidget.AddToViewport` (`self.WidgetPause`) 0))

(event `self.DisplayPlayerHUD`
  (params (CurrentScore :type Integer))
  (`WidgetLayoutLibrary.RemoveAllWidgets`)
  (`UserWidget.AddToViewport` (`self.WidgetHUD`) 0))

(fn `UserConstructionScript`)