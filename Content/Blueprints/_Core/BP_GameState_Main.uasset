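; BP_GameState_Main is the main game state, driving pause and resume from game mode state changes.
; On BeginPlay it broadcasts a reset, binds Paused and GameOver to pause and Playing to unpause, then switches to PLAYING a tick later with zero score.
; Tick calls ReduceTime every frame, and a Quit event exits the game.
; Of its getter functions, only GetGameState returns a value, itself; the rest are empty.
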(event `Initialize`)

(event `self.ReceiveBeginPlay`
  (`parent.ReceiveBeginPlay`)
  (`self.OnGameReset`)
  (add `self.OnPaused` (delegate `Pause Logic`))
  (add `self.OnPlaying` (delegate `Resume Logic`))
  (add `self.OnGameOver` (delegate `Pause Logic`))
  (`KismetSystemLibrary.DelayUntilNextTick`)
  (`self.SetNewGameModeState` "PLAYING"))

(event `Pause Logic` :!signature `self.OnPaused`
  (params (CurrentScore :type Integer))
  (`GameplayStatics.SetGamePaused` true))

(event `Resume Logic` :!signature `self.OnPlaying`
  (params (CurrentScore :type Integer))
  (`GameplayStatics.SetGamePaused` false))

(event `Quit`
  (`KismetSystemLibrary.QuitGame` null "Quit"))

(event `self.ReceiveTick`
  (params (DeltaSeconds :type "Float (single-precision)"))
  (`self.ReduceTime` 1))

(fn `GetCameraManager`
  (returns (CameraManager :type "/Game/Blueprints/Player/Camera/BP_Main_CameraManager Object Reference"))
  (return null))

(fn `GetCoreCameraManager`
  (returns (CameraManager :type "CoreCameraManager Object Reference"))
  (return null))

(fn `GetGameState`
  (returns (GameState :type "/Game/Blueprints/_Core/BP_GameState_Main Object Reference"))
  (return self))

(fn `GetPlayerCharacter`
  (params (PlayerController :type "PlayerController Object Reference"))
  (returns (Character :type "/Game/Blueprints/Player/Pawn/BP_Main_Character Object Reference"))
  (return null))

(fn `GetPlayerController`
  (returns (PlayerController :type "/Game/Blueprints/Player/BP_PlayerController_Main Object Reference"))
  (return null))

(fn `UserConstructionScript`)