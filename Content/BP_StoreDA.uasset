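; Store data object that holds the game's list of store items, each with a price and a purchased flag.
; UpdateStoreItem replaces an entry by removing it by value, then inserting the new data at the same index if the removal succeeds.
; AreStoreItemsAvailable reports whether any unpurchased item costs no more than the given score, stopping at the first match.
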(event `UpdateStoreItem`
  (params (Index :type Integer) (NewData :type "/Game/Str_StoreItem Structure"))
  (bind _storeitems (`self.StoreItems`))
  (bind _returnvalue (`KismetArrayLibrary.Array_RemoveItem` _storeitems (`|GetArrayItem` _storeitems Index)))
  (if _returnvalue
    (`KismetArrayLibrary.Array_Insert` _storeitems NewData Index)))

(fn `AreStoreItemsAvailable`
  (params (CurrentScore :type Integer))
  (returns (AreAvailable :type Boolean))
  (locals (IsAvailable :type Boolean))
  (for _array_element (`self.StoreItems`)
    (if (and (not (`.IsPurchased_12_416812F343DBC70ED80A91B8446600B9` (break `/Game/Str_StoreItem` _array_element))) (<= (`.Price_8_0BEC12194703BF62312E639B14FC6077` (break `/Game/Str_StoreItem` _array_element)) CurrentScore))
      (set `local.IsAvailable` true)
      (break)))
  (return (`local.IsAvailable`)))