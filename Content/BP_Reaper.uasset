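; BP_Reaper is the player character, adding a dash, scythe abilities and an in-game store to its parent class.
; Dashes run on a timeline scaled to the current movement's duration, which interpolates position while velocity is forced forward, and movement input can interrupt them.
; Health combo stage increases briefly enable the store when items are available; IA_Store toggles its widget, pausing the game.
; Abilities activate through components on the held scythe.
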(event `self.ReceiveBeginPlay`
  (bind _healthcombo (`self.HealthCombo`))
  (`parent.ReceiveBeginPlay`)
  (add `self.OnDashUpdate` (delegate `UpdateMovementComponentVel`))
  (bind _returnvalue (`|CreateWidget` "/Game/WBP_Store.WBP_Store_C"))
  (set `self.StoreWidget` _returnvalue)
  (add `HealthCombo.OnStageIncrease` _healthcombo (delegate `EnableStore`))
  (add `HealthCombo.OnStageDecrease` _healthcombo (delegate `DisableStore`)))

(event `EnableStore`
  (params (Stage :type Integer))
  (if (`/Game/BP_StoreDA.AreStoreItemsAvailable` (`/Game/AC_Store.StoreData` (`self.GetComponentByClass` (`GameplayStatics.GetGameMode`) "/Game/AC_Store.AC_Store_C")) Stage)
    (`self.SetStoreEnabled` true)
    (`KismetSystemLibrary.RetriggerableDelay` 4.5)
    (if (not (and (`Widget.IsVisible` (`self.StoreWidget`)) (`self.CanOpenStore`)))
      (`self.SetStoreEnabled` false))))

(event `UpdateMovementComponentVel` :!signature `self.OnDashUpdate`
  (params (ActorTarget :type "Actor Object Reference") (Alpha :type "Float (single-precision)"))
  (bind _charactermovement (`self.CharacterMovement`))
  (set `CharacterMovementComponent.MaxAcceleration` 1000000.0 _charactermovement)
  (set `MovementComponent.Velocity` (* (`self.GetActorForwardVector`) (`CharacterMovementComponent.MaxWalkSpeed` _charactermovement)) _charactermovement))

(event `DisableStore`
  (params (Stage :type Integer))
  (if (not (`/Game/BP_StoreDA.AreStoreItemsAvailable` (`/Game/AC_Store.StoreData` (`self.GetComponentByClass` (`GameplayStatics.GetGameMode`) "/Game/AC_Store.AC_Store_C")) Stage))
    (`self.SetStoreEnabled` false)))

(event `self.ProcessInput`
  (params (InputX :type "Float (single-precision)") (InputY :type "Float (single-precision)") (Target :type "Actor Object Reference"))
  (bind _dashtimeline (`self.DashTimeline`))
  (`parent.ProcessInput` InputX InputY Target)
  (if (`self.CanMove`)
    (if (`TimelineComponent.IsPlaying` _dashtimeline)
      (`TimelineComponent.Stop` _dashtimeline)
      (`self.StopDash`))))

(event `self.ProcessDash`
  (params (Target :type "Actor Object Reference"))
  (bind _dashtimeline (`self.DashTimeline`))
  (bind (_targetposition _successful) (`AbstractMovement.GetDashTargetPosition` (`self.CurrentMovement`) Target (`self.CurXInput`) (`self.CurYInput`)))
  (if (`self.CanMove`)
    (`self.SwitchMovement` Target)
    (set `self.DashStartPos` (`self.K2_GetActorLocation`))
    (set `self.DashTargetPos` _targetposition)
    (if _successful
      (set `self.isDashing` true)
      (set `self.isDashRestrictive` true)
      (`self.OnDashBegin` Target (`self.CurXInput`))
      (`TimelineComponent.SetPlayRate` _dashtimeline (/ (`TimelineComponent.GetTimelineLength` _dashtimeline) (`AbstractMovement.DashDuration` (`self.CurrentMovement`))))
      (bind (_direction _alpha) (`Timeline|DashTimeline` :!via `PlayFromStart`)
        (:`Update`
          (`self.OnDashUpdate` Target _alpha)
          (bind (_newposition _successful_2) (`AbstractMovement.InterpDash` (`self.CurrentMovement`) Target (`self.DashStartPos`) (`self.DashTargetPos`) _alpha))
          (if _successful_2
            (`self.K2_SetActorLocation` _newposition)
            (set `self.isDashRestrictive` (not (`KismetMathLibrary.NearlyEqual_FloatFloat` _alpha (`AbstractMovement.DashOverrideAlpha` (`self.CurrentMovement`)) 0.1)))
            (else
              (`TimelineComponent.Stop` (`self.DashTimeline`))
              (`self.StopDash`))))
        (:`Finished`
          (`self.StopDash`))))))

(event `StopDash`
  (`self.OnDashEnd` null)
  (set `self.isDashing` false)
  (set `self.isDashRestrictive` false)
  (`KismetSystemLibrary.Delay` 0.1)
  (set `CharacterMovementComponent.MaxAcceleration` 2048.0 (`self.CharacterMovement`)))

(event `EnhancedInput|/Game/Input/IA_Store`
  (params (ActionValue :type Boolean) (ElapsedSeconds :type "Float (double-precision)") (TriggeredSeconds :type "Float (double-precision)") (InputAction :type "InputAction Object Reference" :default "/Game/Input/IA_Store.IA_Store"))
  (bind _storewidget (`self.StoreWidget`))
  (bind _storewidget_2 (`self.StoreWidget`))
  (:`Started`
    (if (`Widget.IsVisible` _storewidget)
      (`Widget.RemoveFromParent` _storewidget)
      (`self.SetStoreEnabled` false)
      (`GameplayStatics.SetGamePaused` false)
      (set `PlayerController.bShowMouseCursor` false (`GameplayStatics.GetPlayerController` 0))
      (elif (`self.CanOpenStore`)
        (`UserWidget.AddToViewport` _storewidget_2 0)
        (`/Game/WBP_Store.Initialize` _storewidget_2 (`/Game/BP_StoreDA.StoreItems` (`/Game/AC_Store.StoreData` (`self.GetComponentByClass` (`GameplayStatics.GetGameMode`) "/Game/AC_Store.AC_Store_C"))))
        (`GameplayStatics.SetGamePaused` true)
        (set `PlayerController.bShowMouseCursor` true (`GameplayStatics.GetPlayerController` 0))))))

(event `ActivateAbility`
  (params (`Ability Class` :type "AbsScytheAbility Class Reference"))
  (bind _scythe (`ScytheHand.Scythe` (`self.ScytheHand`)))
  (`AbsScytheAbility.ActivateAbility` (`self.GetComponentByClass` _scythe `Ability Class`) _scythe))

(event `SetStoreEnabled`
  (params (EnableStore :type Boolean))
  (set `self.CanOpenStore` EnableStore)
  (bind _asbp_player_hud (cast `/Game/Blueprints/_Core/BP_PlayerHUD` (`PlayerController.GetHUD` (`/Game/Blueprints/_Core/References/BPFL_References.GetMainPlayerController`))))
  (if (`self.CanOpenStore`)
    (bind _storeenabled (`/Game/UI/WBP_ReaperHUD.StoreEnabled` (`/Game/Blueprints/_Core/BP_PlayerHUD.WidgetHUD` _asbp_player_hud)))
    (`Widget.SetVisibility` _storeenabled "Visible")
    (else
      (`Widget.SetVisibility` _storeenabled "Hidden"))))

(fn `UserConstructionScript`)