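; AC_FreeAim provides a soft-aim check that detects what lies within a cone in front of the main camera.
; CheckSoftAim runs a complex cone trace by channel from the camera location along the camera manager's forward vector, sized by the soft-aim distance and radius.
; It ignores the player pawn and camera manager, draws a one-frame debug shape, and returns the trace result.
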(fn `CheckSoftAim`
  (returns (ReturnValue :type "Array of HitResult Structure"))
  (locals (TraceColor :type "Color Structure" :default (struct :`B` 251 :`G` 249 :`R` 255 :`A` 255)) (TraceHitColor :type "Color Structure" :default (struct :`B` 112 :`G` 99 :`R` 255 :`A` 255)))
  (bind _cameramanager (`/Game/Blueprints/_Core/References/BPFL_References.GetMainCameraManager`))
  (bind _returnvalue (`PlayerCameraManager.GetCameraLocation` _cameramanager))
  (bind _returnvalue_2 (`TraceUtil.ConeTraceByChannel` _cameramanager _returnvalue (+ _returnvalue (* (`Actor.GetActorForwardVector` _cameramanager) (`self.SoftAimDistance`))) (`self.SoftAimRadius`) "TraceTypeQuery3" true (`|MakeArray` (`GameplayStatics.GetPlayerPawn` 0) _cameramanager :!type "Actor Object Reference") "ForOneFrame" true "Circle" (`local.TraceColor`) (`local.TraceHitColor`)))
  (return _returnvalue_2))