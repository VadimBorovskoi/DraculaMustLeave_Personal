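; Enemy targeting component that hands out positions around the player pawn for enemies to occupy.
; On BeginPlay it caches the SC_EnemyTargetPoint components found on player pawn 0.
; GetRandomAvailablePosition shuffles them, then claims and returns the first unoccupied point that differs from the enemy's current one, printing debug names.
; It never frees points itself, and prints a message when none qualify.
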(event `self.ReceiveBeginPlay`
  (set `self.TargetPoints` (`Actor.K2_GetComponentsByClass` (`GameplayStatics.GetPlayerPawn` 0) "/Game/Enemies/SC_EnemyTargetPoint.SC_EnemyTargetPoint_C")))

(fn `GetRandomAvailablePosition`
  (params (Enemy :type "/Game/Enemies/BP_TargetStatic Object Reference"))
  (returns (TargetPosition :type "/Game/Enemies/SC_EnemyTargetPoint Object Reference"))
  (locals (TargetPoint :type "/Game/Enemies/SC_EnemyTargetPoint Object Reference"))
  (bind _targetpoint (`local.TargetPoint`))
  (`KismetArrayLibrary.Array_Shuffle` (`self.TargetPoints`))
  (for _array_element (`self.TargetPoints`)
    (if (not (or (`/Game/Enemies/SC_EnemyTargetPoint.IsOccupied` _array_element) (== (`/Game/Enemies/BP_TargetStatic.OccupiedNavPoint` Enemy) _array_element)))
      (bind _output_get (set `local.TargetPoint` _array_element))
      (`KismetSystemLibrary.PrintString` (`KismetSystemLibrary.GetDisplayName` Enemy) true true (struct :`G` 1.0 :`B` 0.208732 :`A` 1.0) 10.0)
      (`KismetSystemLibrary.PrintString` (`KismetSystemLibrary.GetDisplayName` _output_get) true true (struct :`R` 1.0 :`G` 0.883368 :`B` 0.127325 :`A` 1.0) 10.0)
      (set `/Game/Enemies/SC_EnemyTargetPoint.IsOccupied` true _targetpoint)
      (return _targetpoint)))
  (`KismetSystemLibrary.PrintString` "No Positions Found" true true (struct :`R` 1.0 :`G` 0.034652 :`A` 1.0))
  (return _targetpoint))