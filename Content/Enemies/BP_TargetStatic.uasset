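; BP_TargetStatic is an enemy target pawn that turns in yaw to face the player when play begins.
; BeginPlay also spawns a plain Actor at its own transform and stores it as ActorToFollow.
; UpdateTargetPoint releases the occupied nav point, requests a random free one from the game state's enemy target system, and reports whether it is valid.
; UpdateWalkSpeed sets the FloatingPawnMovement max speed.
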(event `self.ReceiveBeginPlay`
  (bind (_returnvalue_roll _returnvalue_pitch) (`KismetMathLibrary.BreakRotator` (`self.K2_GetActorRotation`)))
  (bind (_returnvalue_roll_2 _returnvalue_pitch_2 _returnvalue_yaw) (`KismetMathLibrary.BreakRotator` (`KismetMathLibrary.FindLookAtRotation` (`self.K2_GetActorLocation`) (`self.K2_GetActorLocation` (`GameplayStatics.GetPlayerPawn` 0)))))
  (`self.K2_SetActorRotation` (`KismetMathLibrary.MakeRotator` _returnvalue_roll _returnvalue_pitch _returnvalue_yaw) true)
  (bind _returnvalue (`|SpawnActorFromClass` "/Script/Engine.Actor" (`self.GetTransform`) "AdjustIfPossibleButAlwaysSpawn" "MultiplyWithRoot" null null))
  (set `self.ActorToFollow` _returnvalue))

(fn `UpdateTargetPoint`
  (returns (Successful :type Boolean))
  (bind _occupiednavpoint (`self.OccupiedNavPoint`))
  (`/Engine/EditorBlueprintResources/StandardMacros.IsValid` _occupiednavpoint
    (:`Is Valid`
      (set `/Game/Enemies/SC_EnemyTargetPoint.IsOccupied` false _occupiednavpoint))
    (:`Is Not Valid`
      _))
  (bind _output_get (set `self.OccupiedNavPoint` (`/Game/Enemies/AC_EnemyTargetSystem.GetRandomAvailablePosition` (`/Game/Blueprints/_Core/BP_GameState_Main.AC_EnemyTargetSystem` (`/Game/Blueprints/_Core/References/BPFL_References.GetMainGameState`)) self)))
  (return (`KismetSystemLibrary.IsValid` _output_get)))

(fn `UpdateWalkSpeed`
  (params (NewSpeed :type "Float (double-precision)"))
  (set `FloatingPawnMovement.MaxSpeed` NewSpeed (`self.FloatingPawnMovement`)))

(fn `UserConstructionScript`)